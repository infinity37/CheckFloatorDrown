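; Level audit actor that, on BeginPlay, finds placed items floating above or sunk into terrain and calls SaveToFile.
; Optional float and drown passes scan ItemClasses, skip ignored actors, and collect offenders in AbnormalActors and their names in Texts.
; The passes call ActorIsFloating and ActorIsDrowning, defined outside this graph.
; BP_ variants, not called here, implement selectable line trace, box trace or bounds tests with an Eps tolerance.
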(event `self.ReceiveBeginPlay`
  (`BlueprintSetLibrary.Set_Clear` (`self.AbnormalActors`))
  (`|ExecutionSequence`
    (:`then_0`
      (if (`self.bCheckFloat`)
        (`self.CheckForFloating`)))
    (:`then_1`
      (if (`self.bCheckDrown`)
        (`self.CheckForDrowning`)))
    (:`then_2`
      (`self.SaveToFile`))))

(fn `BP_ActorIsDrowning`
  (params (CheckActor :type "Actor Object Reference"))
  (returns (IsDrowning :type Boolean))
  (locals (ActorPosition :type "Vector Structure" :default (0.0 0.0 0.0)) (StaticPosition :type "Vector Structure" :default (0.0 0.0 0.0)) (WorldDynamic :type "EObjectTypeQuery Enum" :default "ObjectTypeQuery2") (LowPosition :type "Vector Structure" :default (0.0 0.0 0.0)))
  (bind (_origin _boxextent) (`self.GetActorBounds` CheckActor false false))
  (bind (_origin_2 _boxextent_2) (`self.GetActorBounds` CheckActor false false))
  (bind _eps (`self.eps`))
  (bind _x (.x _origin))
  (bind _y (.y _origin))
  (bind _x_2 (.x (`local.ActorPosition`)))
  (bind _y_2 (.y (`local.ActorPosition`)))
  (bind _returnvalue (`KismetMathLibrary.MakeVector` _x_2 _y_2 -900.0))
  (bind _returnvalue_2 (+ (- (.z _origin) (.z _boxextent)) (* _eps 1.5)))
  (set `local.ActorPosition` (`self.K2_GetActorLocation` CheckActor))
  (switch `ECheckMethods` (`self.mycheckmethod`)
    (:`LineTrace`
      (bind _outhit (`KismetSystemLibrary.LineTraceSingleForObjects` (`KismetMathLibrary.MakeVector` _x_2 _y_2 1000.0) _returnvalue (`self.TerrainTypes`)))
      (set `local.StaticPosition` (`.ImpactPoint` (`GameplayStatics.BreakHitResult` _outhit)))
      (bind _outhit_2 (`KismetSystemLibrary.LineTraceSingleForObjects` _returnvalue (`local.ActorPosition`) (`|MakeArray` (`local.WorldDynamic`))))
      (bind _output_get (set `local.LowPosition` (`.ImpactPoint` (`GameplayStatics.BreakHitResult` _outhit_2))))
      (return (< (.z _output_get) (- (.z (`local.StaticPosition`)) (`self.eps`)))))
    (:`BoxTrace`
      (bind (_outhit_3 _returnvalue_3) (`KismetSystemLibrary.BoxTraceSingleForObjects` :`Start` (`KismetMathLibrary.MakeVector` _x _y _returnvalue_2) :`End` (`KismetMathLibrary.MakeVector` _x _y (- _returnvalue_2 0.1)) :`HalfSize` (`KismetMathLibrary.MakeVector` (.x _boxextent) (.y _boxextent) (/ _eps 2.0)) :`ObjectTypes` (`self.TerrainTypes`) :`DrawDebugType` "Persistent"))
      (return _returnvalue_3))
    (:`BoundCheck`
      (bind _outhit_4 (`KismetSystemLibrary.BoxTraceSingleForObjects` _origin_2 (`KismetMathLibrary.MakeVector` (.x _origin_2) (.y _origin_2) -100.0) _boxextent_2 (struct) (`self.TerrainTypes`)))
      (return (> (.z (`.ImpactPoint` (`GameplayStatics.BreakHitResult` _outhit_4))) (+ (.z (- _origin_2 _boxextent_2)) (`self.eps`)))))))

(fn `BP_ActorIsFloating`
  (params (CheckActor :type "Actor Object Reference"))
  (returns (IsFloating :type Boolean))
  (locals (ActorPosition :type "Vector Structure") (StaticPosition :type "Vector Structure") (WorldDynamic :type "EObjectTypeQuery Enum" :default "ObjectTypeQuery2") (LowPosition :type "Vector Structure" :default (0.0 0.0 0.0)))
  (bind (_origin _boxextent) (`self.GetActorBounds` CheckActor false false))
  (bind (_origin_2 _boxextent_2) (`self.GetActorBounds` CheckActor false false))
  (bind _actorposition (`local.ActorPosition`))
  (bind _x (.x _origin))
  (bind _y (.y _origin))
  (bind _returnvalue (/ (`self.eps`) 2.0))
  (bind _returnvalue_2 (- (- (.z _origin) (.z _boxextent)) _returnvalue))
  (set `local.ActorPosition` (`self.K2_GetActorLocation` CheckActor))
  (switch `ECheckMethods` (`self.mycheckmethod`)
    (:`LineTrace`
      (bind _outhit (`KismetSystemLibrary.LineTraceSingleForObjects` :`Start` _actorposition :`End` (`KismetMathLibrary.MakeVector` (.x _actorposition) (.y _actorposition) -1000.0) :`ObjectTypes` (`self.TerrainTypes`) :`DrawDebugType` "Persistent"))
      (bind _output_get (set `local.StaticPosition` (`.ImpactPoint` (`GameplayStatics.BreakHitResult` _outhit))))
      (bind _outhit_2 (`KismetSystemLibrary.LineTraceSingleForObjects` :`Start` _output_get :`End` (`local.ActorPosition`) :`ObjectTypes` (`|MakeArray` (`local.WorldDynamic`)) :`DrawDebugType` "Persistent"))
      (bind _output_get_2 (set `local.LowPosition` (`.ImpactPoint` (`GameplayStatics.BreakHitResult` _outhit_2))))
      (return (and (not (== _output_get_2 (0.0 0.0 0.0))) (> (.z _output_get_2) (+ (.z (`local.StaticPosition`)) (`self.eps`))))))
    (:`BoxTrace`
      (bind (_outhit_3 _returnvalue_3) (`KismetSystemLibrary.BoxTraceSingleForObjects` :`Start` (`KismetMathLibrary.MakeVector` _x _y _returnvalue_2) :`End` (`KismetMathLibrary.MakeVector` _x _y (- _returnvalue_2 0.1)) :`HalfSize` (`KismetMathLibrary.MakeVector` (.x _boxextent) (.y _boxextent) _returnvalue) :`ObjectTypes` (`self.TerrainTypes`) :`DrawDebugType` "Persistent"))
      (return (not _returnvalue_3)))
    (:`BoundCheck`
      (bind _outhit_4 (`KismetSystemLibrary.BoxTraceSingleForObjects` _origin_2 (`KismetMathLibrary.MakeVector` (.x _origin_2) (.y _origin_2) -100.0) _boxextent_2 (struct) (`self.TerrainTypes`)))
      (return (< (.z (`.ImpactPoint` (`GameplayStatics.BreakHitResult` _outhit_4))) (- (.z (- _origin_2 _boxextent_2)) (`self.eps`)))))))

(fn `CheckForDrowning`
  (for _array_element (`self.ItemClasses`)
    (bind _outactors (`GameplayStatics.GetAllActorsOfClass` _array_element))
    (for _array_element_2 _outactors
      (if (not (`BlueprintSetLibrary.Set_Contains` (`self.ActorsToIgnore`) _array_element_2))
        (bind _isdrowning (`self.BP_ActorIsDrowning` _array_element_2))
        (if _isdrowning
          (`BlueprintSetLibrary.Set_Add` (`self.AbnormalActors`) _array_element_2)
          (`KismetArrayLibrary.Array_Add` (`self.texts`) (`KismetSystemLibrary.GetDisplayName` _array_element_2)))))))

(fn `CheckForFloating`
  (for _array_element (`self.ItemClasses`)
    (bind _outactors (`GameplayStatics.GetAllActorsOfClass` _array_element))
    (for _array_element_2 _outactors
      (if (not (`BlueprintSetLibrary.Set_Contains` (`self.ActorsToIgnore`) _array_element_2))
        (bind _isfloating (`self.BP_ActorIsFloating` _array_element_2))
        (if _isfloating
          (`BlueprintSetLibrary.Set_Add` (`self.AbnormalActors`) _array_element_2)
          (`KismetArrayLibrary.Array_Add` (`self.texts`) (`KismetSystemLibrary.GetDisplayName` _array_element_2)))))))

(fn `UserConstructionScript`)